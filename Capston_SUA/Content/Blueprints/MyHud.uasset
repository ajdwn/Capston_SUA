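; MyHud is a HUD Blueprint that displays the player sedan's forward speed and current gear.
; On each DrawHUD it casts the owning pawn to BP_Sedan_2 and reads its vehicle movement component, converting speed from cm/s to km/h.
; It creates a new UI_TutoPlay widget on every draw, fills its Speed and Gear texts, and adds it to the viewport without removing earlier ones.
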(event EventDrawHUD
  (params (SizeX :type Integer) (SizeY :type Integer))
  (bind _asbp_sedan_2 (Utilities|Casting|CastToBP_Sedan_2 (Class|HUD|GetOwningPawn)))
  (bind _returnvalue (UserInterface|CreateWidget "/Game/Graphic/Scene/UI_TutoPlay.UI_TutoPlay_C"))
  (Rendering|Components|TextRender|SetText (Variables|/Game/Graphic/Scene/UI_TutoPlay.UI_TutoPlay_C|Getspeed _returnvalue) (Utilities|Text|ToText(Float) (* (Vehicle|GetForwardSpeed (Variables|/Script/ChaosVehicles.WheeledVehiclePawn|GetVehicleMovementComponent _asbp_sedan_2)) 0.036) "HalfToEven"))
  (Rendering|Components|TextRender|SetText (Variables|/Game/Graphic/Scene/UI_TutoPlay.UI_TutoPlay_C|Getgear _returnvalue) (Utilities|Text|ToText(Integer) (Class|ChaosVehicleMovementComponent|GetCurrentGear (Variables|/Script/ChaosVehicles.WheeledVehiclePawn|GetVehicleMovementComponent _asbp_sedan_2))))
  (UserInterface|Viewport|AddtoViewport _returnvalue 0))

(fn ConstructionScript)